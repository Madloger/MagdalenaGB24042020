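; Turret base that tracks the nearest actor inside its sphere and triggers a fire event at it.
; Sphere overlaps maintain the target list, from which FineNearTarget picks by distance.
; Tick interpolates TurretRot toward that target without applying it to a component, calling OnFire once nearly aligned and IsAllowFire passes.
; OnFire is empty, and the cooldown adds FireInterval twice, so shots are spaced at double that value.
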(event OnComponentBeginOverlap(Sphere)
  (params (OverlappedComponent :type Primitive%20Component%20Object%20Reference) (OtherActor :type Actor%20Object%20Reference) (OtherComp :type Primitive%20Component%20Object%20Reference) (OtherBodyIndex :type Integer) (bFromSweep :type Boolean) (SweepResult :type Hit%20Result%20Structure%20%28by%20ref%29))
  (Utilities|Array|AddUnique (Variables|Default|GetTargets) OtherActor))

(event OnComponentEndOverlap(Sphere)
  (params (OverlappedComponent :type Primitive%20Component%20Object%20Reference) (OtherActor :type Actor%20Object%20Reference) (OtherComp :type Primitive%20Component%20Object%20Reference) (OtherBodyIndex :type Integer))
  (Utilities|Array|RemoveItem (Variables|Default|GetTargets) OtherActor))

(event Custom|OnFire
  (params (Target :type Actor%20Object%20Reference)))

(event EventBeginPlay)

(event Collision|EventActorBeginOverlap
  (params (OtherActor :type Actor%20Object%20Reference)))

(event EventTick
  (params (DeltaSeconds :type Float%20%28single-precision%29))
  (bind _outactor (CallFunction|FineNearTarget))
  (bind _returnvalue (Transformation|GetActorLocation))
  (bind _returnvalue_2 (Transformation|GetActorLocation _outactor))
  (bind _returnvalue_3 (Math|Rotator|FindLookatRotation _returnvalue _returnvalue_2))
  (Utilities|IsValid _outactor
    (:Is%20Valid
      (bind _output_get (Variables|Default|SetTurretRot (Math|Interpolation|RInterpTo (Variables|Default|GetTurretRot) _returnvalue_3 DeltaSeconds (Variables|Default|GetRotSpeed))))
      (if (Math|Rotator|Equal(Rotator) _output_get _returnvalue_3 1.0)
        (if (CallFunction|IsAllowFire)
          (CallFunction|OnFire _outactor))))))

(fn ConstructionScript)

(fn FineNearTarget
  (for _array_element (Variables|Default|GetTargets)
    (Utilities|IsValid _array_element
      (:Is%20Valid
        (if (< (Math|Vector|Distance(Vector) (Transformation|GetActorLocation _array_element) (Transformation|GetActorLocation)) (LocalVariables|GetDistance))
          (LocalVariables|SetDistance (Math|Vector|Distance(Vector) (Transformation|GetActorLocation _array_element) (Transformation|GetActorLocation)))
          (LocalVariables|SetLastTarget _array_element)))))
  (return (LocalVariables|GetLastTarget)))

(fn IsAllowFire
  (bind _returnvalue (Utilities|Time|GetTimeSeconds))
  (bind _fireinterval (Variables|Default|GetFireInterval))
  (if (< (+ (Variables|Default|GetLastShot) _fireinterval) _returnvalue)
    (Variables|Default|SetLastShot (+ _returnvalue _fireinterval))
    (return true)
    (else
      (return false))))