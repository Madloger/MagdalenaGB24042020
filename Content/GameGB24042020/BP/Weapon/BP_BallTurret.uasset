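; Ball turret weapon Blueprint that rotates to an aim rotation and fires through a projectile component.
; Each Tick, after the parent's Tick, it sets the Scene component's world rotation directly to TurretRot, which this graph reads but never computes.
; The OnFire event delegates shooting to BPProjFairComponent by calling its Fair function.
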(event EventBeginPlay
  (|CallParentFunction) ; This node is disabled and will not be called.\nDrag off pins to build functionality.
)

(event Collision|EventActorBeginOverlap
  (params (OtherActor :type Actor%20Object%20Reference))
  (|CallParentFunction OtherActor) ; This node is disabled and will not be called.\nDrag off pins to build functionality.
)

(event EventTick
  (params (DeltaSeconds :type Float%20%28single-precision%29))
  (|CallParentFunction DeltaSeconds)
  (Transformation|SetWorldRotation (Variables|Default|GetScene) (Variables|Default|GetTurretRot) false false))

(event EventOnFire
  (params (Target :type Actor%20Object%20Reference))
  (Default|Fair (Variables|Default|GetBP_ProjFairComponent)))

(fn ConstructionScript
  (|CallParentFunction))