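; Turret projectile Blueprint that deals radial damage with falloff at its location.
; Launch stores the damage amount and makes the collision sphere ignore the instigator while moving.
; A projectile bounce explodes it only when IsExplodeOnHit is set, while a projectile stop always explodes it.
; Explode applies the damage and sets a short life span instead of destroying the actor immediately.
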(event OnProjectileBounce(ProjectileMovement)
  (params (ImpactResult :type Hit%20Result%20Structure%20%28by%20ref%29) (ImpactVelocity :type Vector%20%28by%20ref%29 :default "0, 0, 0"))
  (if (Variables|Default|GetIsExplodeOnHit)
    (CallFunction|Explode)))

(event OnProjectileStop(ProjectileMovement)
  (params (ImpactResult :type Hit%20Result%20Structure%20%28by%20ref%29))
  (CallFunction|Explode))

(fn ConstructionScript)

(fn Explode
  (Class|GameplayStatics|ApplyRadialDamagewithFalloff (Variables|Default|GetDamage) 0.0 (Transformation|GetActorLocation) (Variables|Default|GetBaseRadius) (Variables|Default|GetFolloyRadius) 0.0 0 0 self 0 "ECC_Pawn")
  (Actor|SetLifeSpan 3.0))

(fn Launch
  (params (InDamage :type Float%20%28single-precision%29) (Instigator :type Actor%20Object%20Reference))
  (Variables|Default|SetDamage InDamage)
  (Collision|IgnoreActorwhenMoving (Variables|Default|GetSphere) Instigator true))