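; BP_ProjFairComponent is a turret component that fires projectiles.
; Its Fair override calls the parent, then spawns an actor of ProjClass at the component's world transform, regardless of collisions.
; It launches that projectile with the component's Damage and passes the owning actor as instigator.
; The event graph holds only disabled stubs, so all of its logic lives in Fair.
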(event EventBeginPlay
  (|CallParentFunction) ; This node is disabled and will not be called.\nDrag off pins to build functionality.
)

(event EventTick
  (params (DeltaSeconds :type Float%20%28single-precision%29))
  (|CallParentFunction DeltaSeconds) ; This node is disabled and will not be called.\nDrag off pins to build functionality.
)

(fn Fair
  (|CallParentFunction)
  (bind _returnvalue (Game|SpawnActorfromClass (Variables|Default|GetProjClass) (Transformation|GetWorldTransform) "AlwaysSpawn" 0 0))
  (Default|Launch _returnvalue (Variables|Default|GetDamage) (Components|GetOwner)))